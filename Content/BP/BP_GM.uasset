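; BP_GM bridges a Pixel Streaming web UI to BP_zSpaceManager, which drives a robot simulation.
; On BeginPlay it finds the manager and binds the player controller's PixelStreamerInputComponent input event.
; Each JSON message's Category and Item drive robot reset, six joint rotations, hardcoded placeholder file paths, IK toggle, joint export and target scrubbing.
; Reset replies with initial rotations as JSON; joint and target setters run on every message.
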(event `self.ReceiveBeginPlay`
  ;[1 1 1] Set Manager Nachi
  (bind _returnvalue (`GameplayStatics.GetActorOfClass` "/Game/BP/BP_zSpaceManager.BP_zSpaceManager_C"))
  (`/Engine/EditorBlueprintResources/StandardMacros.IsValid` _returnvalue
    (:`Is Valid`
      (set `self.zSpaceManager` _returnvalue)
      ;[1 1 1] Bind Web Events
      (bind _output_get (set `self.PixelStreamComp` (`self.GetComponentByClass` (`GameplayStatics.GetPlayerController` 0) "/Script/PixelStreaming.PixelStreamerInputComponent")))
      (add `PixelStreamerInputComponent.OnInputEvent` _output_get (delegate `UI_Client_Interaction`)))))

(event `UI_Client_Interaction`
  (params (Descriptor :type String))
  ;[1 1 1] Bind Web Events
  (bind _output_get (set `self.Descriptor` Descriptor))
  (`self.UI_Events` _output_get))

(event `UI_Events`
  (params (Descriptor :type String))
  (bind _zspacemanager (`self.zSpaceManager`))
  (bind _zspacemanager_2 (`self.zSpaceManager`))
  (`|ExecutionSequence`
    (:`then_0`
      (bind (_returnvalue _success) (`self.CheckJSONValue` "0" (`self.Descriptor`)))
      (if _success
        (`zSpaceManager.ResetRobot` _zspacemanager_2)
        (set `self.sendDescriptor` "")
        (for (_array_element _array_index) (`zSpaceManager.initialRotations` _zspacemanager_2)
          (set `self.sendDescriptor` (`PixelStreamerInputComponent.AddJsonStringValue` (`self.PixelStreamComp`) (`self.sendDescriptor`) (`KismetStringLibrary.Concat_StrStr` "j" (`KismetStringLibrary.Conv_IntToString` _array_index)) (`KismetStringLibrary.Conv_DoubleToString` _array_element))))
        (`PixelStreamerInputComponent.SendPixelStreamingResponse` (`self.PixelStreamComp`) (`self.sendDescriptor`))))
    (:`then_1`
      (`self.SetJointsValue` (`self.Descriptor`))
      (`zSpaceManager.SetJointRotations` (`self.zSpaceManager`) (`self.J1`) (`self.J2`) (`self.J3`) (`self.J4`) (`self.J5`) (`self.J6`)))
    (:`then_2`
      (bind (_returnvalue_2 _success_2) (`self.CheckJSONValue` "30" (`self.Descriptor`)))
      (if _success_2
        (if (== _returnvalue_2 1.0)
          (`zSpaceManager.SetObjectPath` (`self.zSpaceManager`) "C:/geometry.obj") ; TODO: bind to FTP file transfer
          (else
            (`zSpaceManager.SetToolPath` (`self.zSpaceManager`) "C:/path.txt") ; TODO: Change for FTP
          ))))
    (:`then_3`
      (`self.ComputeIK`))
    (:`then_4`
      (bind _returnvalue_3 (`self.CheckJSONValue` "21" (`self.Descriptor`)))
      (bind _returnvalue_4 (`zSpaceManager.GetTargetCount` _zspacemanager))
      (`zSpaceManager.SetTargetCounter` _zspacemanager (`KismetMathLibrary.Round` (* (- _returnvalue_4 1) _returnvalue_3))))))

(fn `CheckJSONValue`
  (params (CategoryString :type String) (Descriptor :type String))
  (returns (ReturnValue :type "Float (double-precision)") (Success :type Boolean))
  (bind _pixelstreamcomp (`self.PixelStreamComp`))
  (bind (_stringvalue _success) (`PixelStreamerInputComponent.GetJsonStringValue` _pixelstreamcomp Descriptor "Category"))
  (bind _returnvalue (`KismetStringLibrary.EqualEqual_StrStr` _stringvalue CategoryString))
  (if _success
    (if _returnvalue
      _
      (else
        _)))
  (return (`KismetStringLibrary.Conv_StringToDouble` (`PixelStreamerInputComponent.GetJsonStringValue` _pixelstreamcomp Descriptor "Item")) _returnvalue))

(fn `ComputeIK`
  (bind _zspacemanager (`self.zSpaceManager`))
  (bind (_returnvalue _success) (`self.CheckJSONValue` "20" (`self.Descriptor`)))
  (if _success
    (if (== _returnvalue 0.0)
      (bind _output_get (set `self.isIk` (not (`self.isIk`))))
      (`zSpaceManager.SetRobotIK` _zspacemanager _output_get)
      (elif (== _returnvalue 1.0)
        (`zSpaceManager.ExportJointRotations` _zspacemanager) ; TODO: send pixel streaming responce
      ))))

(fn `SetJointsValue`
  (params (InputPin :type String))
  (`|ExecutionSequence`
    (:`then_0`
      (bind (_returnvalue _success) (`self.CheckJSONValue` "10" InputPin))
      (if _success
        (set `self.J1` _returnvalue)))
    (:`then_1`
      (bind (_returnvalue_2 _success_2) (`self.CheckJSONValue` "11" InputPin))
      (if _success_2
        (set `self.J2` _returnvalue_2)))
    (:`then_2`
      (bind (_returnvalue_3 _success_3) (`self.CheckJSONValue` "12" InputPin))
      (if _success_3
        (set `self.J3` _returnvalue_3)))
    (:`then_3`
      (bind (_returnvalue_4 _success_4) (`self.CheckJSONValue` "13" InputPin))
      (if _success_4
        (set `self.J4` _returnvalue_4)))
    (:`then_4`
      (bind (_returnvalue_5 _success_5) (`self.CheckJSONValue` "14" InputPin))
      (if _success_5
        (set `self.J5` _returnvalue_5)))
    (:`then_5`
      (bind (_returnvalue_6 _success_6) (`self.CheckJSONValue` "15" InputPin))
      (if _success_6
        (set `self.J6` _returnvalue_6)))))

(fn `UserConstructionScript`)